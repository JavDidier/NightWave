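; Interactable battery pickup that recharges the player character's battery and consumes itself.
; On Interact, if the player's battery is below its maximum, it sets the charge to a fixed value capped at that maximum and passes it to GestionBattery.
; It then destroys itself, flags battery use, sets the player's spotlight intensity, and loops back to the charge check.
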(event `/Game/_Game/Ui/BPI_Interface.Interact`
  (bind _asl1_player_character (cast `/Game/_Game/_GameBP/Level1/L1_PlayerCharacter` (`GameplayStatics.GetPlayerCharacter` 0)))
  (if (< (`/Game/_Game/_GameBP/Level1/L1_PlayerCharacter.battery` _asl1_player_character) (`/Game/_Game/_GameBP/Level1/L1_PlayerCharacter.batteryMax` _asl1_player_character)) :!label _label
    (bind _output_get (set `/Game/_Game/_GameBP/Level1/L1_PlayerCharacter.battery` (`KismetMathLibrary.FClamp` 100.0 0.0 (`/Game/_Game/_GameBP/Level1/L1_PlayerCharacter.batteryMax` _asl1_player_character)) _asl1_player_character))
    (`/Game/_Game/_GameBP/Level1/L1_PlayerCharacter.gestionBattery` _asl1_player_character _output_get)
    (`self.K2_DestroyActor`)
    (set `/Game/_Game/_GameBP/Level1/L1_PlayerCharacter.useBattery` true _asl1_player_character)
    (`LightComponent.SetIntensity` (`/Game/_Game/_GameBP/Level1/L1_PlayerCharacter.SpotLight` _asl1_player_character) 50.0)
    (goto _label)))

(fn `UserConstructionScript`)