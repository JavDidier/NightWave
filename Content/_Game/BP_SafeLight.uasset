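; BP_SafeLight is a safe-zone light that calms the player's fear and turns enemies back to patrolling.
; When BoxSafeLight is entered, a BP_ennemie is sent to patrol, while an L1_PlayerCharacter is flagged InSafeZone, has its fear-increase timer cleared and starts lowering fear (Peur).
; When the player leaves the box, the flag resets, the decrease timer is cleared and fear starts rising again.
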(event `self.BoxSafeLight.OnComponentBeginOverlap`
  (params (OverlappedComponent :type "PrimitiveComponent Object Reference") (OtherActor :type "Actor Object Reference") (OtherComp :type "PrimitiveComponent Object Reference") (OtherBodyIndex :type Integer) (bFromSweep :type Boolean) (SweepResult :type "HitResult Structure (by ref)"))
  (`|ExecutionSequence`
    (:`then_0`
      (bind _asbp_ennemie (cast `/Game/_Game/Ennemies/BP_ennemie` OtherActor))
      (`/Game/_Game/Ennemies/BP_ennemie.patrouilleEnnemi` _asbp_ennemie))
    (:`then_1`
      (bind _asl1_player_character (cast `/Game/_Game/_GameBP/Level1/L1_PlayerCharacter` OtherActor))
      (set `/Game/_Game/_GameBP/Level1/L1_PlayerCharacter.inSafeZone?` true _asl1_player_character)
      (`/Game/_Game/_GameBP/Level1/L1_PlayerCharacter.clearTimer` _asl1_player_character (`/Game/_Game/_GameBP/Level1/L1_PlayerCharacter.AugmentePeurRef` _asl1_player_character))
      (`/Game/_Game/_GameBP/Level1/L1_PlayerCharacter.DescendrePeur` _asl1_player_character))))

(event `self.BoxSafeLight.OnComponentEndOverlap`
  (params (OverlappedComponent :type "PrimitiveComponent Object Reference") (OtherActor :type "Actor Object Reference") (OtherComp :type "PrimitiveComponent Object Reference") (OtherBodyIndex :type Integer))
  (bind _asl1_player_character (cast `/Game/_Game/_GameBP/Level1/L1_PlayerCharacter` OtherActor))
  (bind _output_get (set `/Game/_Game/_GameBP/Level1/L1_PlayerCharacter.inSafeZone?` false _asl1_player_character))
  (`/Game/_Game/_GameBP/Level1/L1_PlayerCharacter.clearTimer` _asl1_player_character (`/Game/_Game/_GameBP/Level1/L1_PlayerCharacter.DiminuePeurRef` _asl1_player_character))
  (`/Game/_Game/_GameBP/Level1/L1_PlayerCharacter.AugmenterPeur` _asl1_player_character))

(fn `UserConstructionScript`)