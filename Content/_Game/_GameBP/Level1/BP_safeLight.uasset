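; BP_safeLight is a Level 1 trigger that sends enemies to patrol when the player enters it with the flashlight on.
; It caches the L1_PlayerCharacter on BeginPlay.
; On Box overlap it checks FlashlightAllume and that the player is the overlapping actor, then calls PatrouilleEnnemi on every BP_ennemie in the world.
; The flashlight is only checked when an overlap begins.
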(event `self.ReceiveBeginPlay`
  (bind _asl1_player_character (cast `/Game/_Game/_GameBP/Level1/L1_PlayerCharacter` (`GameplayStatics.GetPlayerCharacter` 0)))
  (set `self.As L1 Player Character` _asl1_player_character))

(event `self.Box.OnComponentBeginOverlap`
  (params (OverlappedComponent :type "PrimitiveComponent Object Reference") (OtherActor :type "Actor Object Reference") (OtherComp :type "PrimitiveComponent Object Reference") (OtherBodyIndex :type Integer) (bFromSweep :type Boolean) (SweepResult :type "HitResult Structure (by ref)"))
  (if (`/Game/_Game/_GameBP/Level1/L1_PlayerCharacter.flashlightAllume?` (`self.As L1 Player Character`))
    (if (== OtherActor (`GameplayStatics.GetPlayerCharacter` 0))
      (bind _outactors (`GameplayStatics.GetAllActorsOfClass` "/Game/_Game/Ennemies/BP_ennemie.BP_ennemie_C"))
      (for _array_element _outactors
        (`/Game/_Game/Ennemies/BP_ennemie.patrouilleEnnemi` _array_element)))))

(fn `UserConstructionScript`)