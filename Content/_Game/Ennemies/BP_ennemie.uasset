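; BP_ennemie is an enemy pawn, animated as a werewolf, that patrols at random and chases the player on sight.
; Patrol loops AIMoveTo toward random reachable points, restarting on success or failure.
; PawnSensing triggers a growl and chase behind a DoOnce, which resets only if the chase fails.
; Reaching the player plays a breath sound and punch animation, then prints a death message without applying damage.
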(event `self.ReceiveBeginPlay`
  (`|ExecutionSequence`
    (:`then_0`
      (bind _asl1_player_character (cast `/Game/_Game/_GameBP/Level1/L1_PlayerCharacter` (`GameplayStatics.GetPlayerCharacter` 0)))
      (set `self.RefJoueur` _asl1_player_character))
    (:`then_1`
      (`self.patrouilleEnnemi`))))

(event `patrouilleEnnemi`
  (`|AIMoveTo` self (`NavigationSystemV1.K2_GetRandomReachablePointInRadius` (`self.K2_GetActorLocation` self) 10000.0 null null) null 50.0
    (:`OnSuccess`
      _)
    (:`OnFail`
      _))
  (`self.patrouilleEnnemi` self))

(event `self.PawnSensing.OnSeePawn`
  (params (Pawn :type "Pawn Object Reference"))
  (bind _returnvalue (`self.K2_GetActorLocation` self))
  (`/Engine/EditorBlueprintResources/StandardMacros.DoOnce` false :!label _label
    (:`Completed`
      (`GameplayStatics.PlaySoundAtLocation` "/Game/_Game/Sounds/creatures/mixkit-angry-dragon-growl-309.mixkit-angry-dragon-growl-309" _returnvalue (struct) 0.5 1.0 0.0 null null null null)
      (`|AIMoveTo` self (0.0 0.0 0.0) (`GameplayStatics.GetPlayerCharacter` 0) 50.0
        (:`OnSuccess`
          (`GameplayStatics.PlaySoundAtLocation` "/Game/_Game/Sounds/creatures/mixkit-monster-breath-1978.mixkit-monster-breath-1978" _returnvalue (struct) 1.0 1.0 0.0 null null null null)
          (`SkeletalMeshComponent.PlayAnimation` (`self.Mesh`) "/Game/Werewolf/Animation/Anim_werewolf_punch.Anim_werewolf_punch" false)
          (`KismetSystemLibrary.Delay` 2.0)
          (`KismetSystemLibrary.PrintText` "T'es Mort :!!"))
        (:`OnFail`
          (`|ExecutionSequence`
            (:`then_0`
              (goto _label :!via `Reset`))
            (:`then_1`
              (`KismetSystemLibrary.PrintString` "Echoiuéééé"))))))))

(fn `UserConstructionScript`)